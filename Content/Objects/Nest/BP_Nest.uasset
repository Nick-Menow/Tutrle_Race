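; BP_Nest is a color-coded portal nest that spawns turtles and sends them walking.
; The construction script uses NumPortal to pick the green, yellow or blue portal effect, its yaw, and world-space offsets for the spawn and target points.
; SpawnTurtle spawns T_1, messages it the target and portal number, and plays a creation sound.
; Actors overlapping the Box receive a message to walk to EndPoint.
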(event `/Game/TutrlesBP/MEssage.Spawn Turtle`
  (params (Number :type Integer) (NewParam :type Integer))
  (bind _returnvalue (`SceneComponent.K2_GetComponentLocation` (`self.Scene`)))
  (bind _returnvalue_2 (`|SpawnActorFromClass` "/Game/TutrlesBP/T_1.T_1_C" (`KismetMathLibrary.MakeTransform` (`SceneComponent.K2_GetComponentLocation` (`self.Scene_Spawn`))) "Undefined" "OverrideRootScale" null null))
  (`/Engine/EditorBlueprintResources/StandardMacros.IsValid` _returnvalue_2
    (:`Is Valid`
      (message `/Game/TutrlesBP/MEssage.Start Create and Moving` _returnvalue_2 _returnvalue (`self.NumPortal`))
      (`GameplayStatics.PlaySoundAtLocation` "/Game/Sounds/Sound_Turtle_Create_Cue.Sound_Turtle_Create_Cue" _returnvalue (struct) 1.0 1.0 0.0 null null null))))

(event `self.Box.OnComponentBeginOverlap`
  (params (OverlappedComponent :type "PrimitiveComponent Object Reference") (OtherActor :type "Actor Object Reference") (OtherComp :type "PrimitiveComponent Object Reference") (OtherBodyIndex :type Integer) (bFromSweep :type Boolean) (SweepResult :type "HitResult Structure (by ref)"))
  (message `/Game/TutrlesBP/MEssage.Start Walking to Point` OtherActor (`self.EndPoint`) (`self.NumPortal`)))

(fn `UserConstructionScript`
  (bind _returnvalue (- (`self.NumPortal`) 1))
  (bind _returnvalue_2 (`SceneComponent.K2_GetComponentLocation` (`self.DefaultSceneRoot`)))
  (bind (_returnvalue_roll _returnvalue_pitch _returnvalue_yaw) (`KismetMathLibrary.BreakRotator` (`SceneComponent.K2_GetComponentRotation` (`self.DefaultSceneRoot`))))
  (`ParticleSystemComponent.SetTemplate` (`self.Portal`) (select `int` _returnvalue :`0` "/Game/Portal/Portal_Green.Portal_Green" :`1` "/Game/Portal/Portal_Yellow.Portal_Yellow" :`2` "/Game/Portal/Portal_Blue.Portal_Blue" :!type "ParticleSystem Object Reference"))
  (`SceneComponent.K2_SetWorldLocation` (`self.Scene`) (+ _returnvalue_2 (select `int` _returnvalue :`0` (0.0 -200.0 0.0) :`1` (200.0 0.0 0.0) :`2` (200.0 0.0 0.0) :!type "Vector Structure")) false false)
  (`SceneComponent.K2_SetWorldLocation` (`self.Scene_Spawn`) (+ _returnvalue_2 (select `int` _returnvalue :`0` (0.0 10.0 0.0) :`1` (-10.0 0.0 0.0) :`2` (-10.0 0.0 0.0) :!type "Vector Structure")) false false)
  (`SceneComponent.K2_SetWorldRotation` (`self.Portal`) (`KismetMathLibrary.MakeRotator` 0.0 0.0 (+ _returnvalue_yaw (select `int` _returnvalue :`0` 0.0 :`1` -90.0 :`2` -90.0 :!type "Float (single-precision)"))) false false))