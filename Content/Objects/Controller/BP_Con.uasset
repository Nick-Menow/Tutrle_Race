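; BP_Con is a numbered, color-coded button object that links the first-person player to its assigned SpawnNest while they stand in range.
; The construction script writes Num to a text render and picks a green, yellow or blue button material from it.
; Sphere overlap stores SpawnNest and Num on the character if its Tumbler slot is empty and shows a second text.
; Leaving clears both and hides that text, only if this nest is the stored one.
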(event `self.ReceiveBeginPlay`)

(event `self.Sphere.OnComponentBeginOverlap`
  (params (OverlappedComponent :type "PrimitiveComponent Object Reference") (OtherActor :type "Actor Object Reference") (OtherComp :type "PrimitiveComponent Object Reference") (OtherBodyIndex :type Integer) (bFromSweep :type Boolean) (SweepResult :type "HitResult Structure (by ref)"))
  (bind _asfirst_person_character (cast `/Game/FirstPersonBP/Blueprints/FirstPersonCharacter` (`GameplayStatics.GetPlayerCharacter` 0) :!pure true))
  (`/Engine/EditorBlueprintResources/StandardMacros.IsValid` (`/Game/FirstPersonBP/Blueprints/FirstPersonCharacter.Tumbler` _asfirst_person_character)
    (:`Is Not Valid`
      (set `/Game/FirstPersonBP/Blueprints/FirstPersonCharacter.Tumbler` (`self.Spawn_nest`) _asfirst_person_character)
      (set `/Game/FirstPersonBP/Blueprints/FirstPersonCharacter.IndexTumbler` (`self.Num`) _asfirst_person_character)
      (`SceneComponent.SetVisibility` (`self.TextRender1`) true false))))

(event `self.Sphere.OnComponentEndOverlap`
  (params (OverlappedComponent :type "PrimitiveComponent Object Reference") (OtherActor :type "Actor Object Reference") (OtherComp :type "PrimitiveComponent Object Reference") (OtherBodyIndex :type Integer))
  (bind _asfirst_person_character (cast `/Game/FirstPersonBP/Blueprints/FirstPersonCharacter` (`GameplayStatics.GetPlayerCharacter` 0) :!pure true))
  (bind _tumbler (`/Game/FirstPersonBP/Blueprints/FirstPersonCharacter.Tumbler` _asfirst_person_character))
  (if (and (`KismetSystemLibrary.IsValid` _tumbler) (== _tumbler (`self.Spawn_nest`)))
    (set `/Game/FirstPersonBP/Blueprints/FirstPersonCharacter.Tumbler` null _asfirst_person_character)
    (set `/Game/FirstPersonBP/Blueprints/FirstPersonCharacter.IndexTumbler` 0 _asfirst_person_character)
    (`SceneComponent.SetVisibility` (`self.TextRender1`) false false)))

(fn `UserConstructionScript`
  (bind _num (`self.Num`))
  (`TextRenderComponent.K2_SetText` (`self.TextRender`) (`KismetTextLibrary.Conv_IntToText` _num))
  (`PrimitiveComponent.SetMaterial` (`self.Button`) 0 (select `int` (- _num 1) :`0` "/Game/Objects/Controller/M_Green.M_Green" :`1` "/Game/Objects/Controller/M_Yellow.M_Yellow" :`2` "/Game/Objects/Controller/M_Blue.M_Blue" :!type "MaterialInterface Object Reference")))